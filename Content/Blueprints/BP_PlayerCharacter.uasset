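; Side-view player character with flipbook animation, horizontal movement, jumping and interaction with nearby objects.
; Enhanced Input moves it along the actor's forward axis and rotates only the sprite to face the travel direction.
; An IsJumping flag keeps run and idle flipbooks from replacing the jump animation until landing resets it to idle.
; Pressing E calls Interact on every BP_Interactable overlapping its Sphere.
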(event Input|EnhancedActionEvents|EnhancedInputActionIA_Move
  (params (ActionValue :type Float%20%28double-precision%29) (ElapsedSeconds :type Float%20%28double-precision%29) (TriggeredSeconds :type Float%20%28double-precision%29) (InputAction :type Input%20Action%20Object%20Reference :default "/Game/Inputs/InputActions/IA_Move.IA_Move"))
  (:Triggered
    (Pawn|Input|AddMovementInput (Transformation|GetActorForwardVector) ActionValue false)
    (if (Variables|Default|GetIsJumping?)
      _
      (else
        (Sprite|SetFlipbook (Variables|Default|GetSprite) "/Game/Art/Character/FB_Run.FB_Run")))
    (if (> ActionValue 0.0)
      (Transformation|SetRelativeRotation (Variables|Default|GetSprite) "0, 0, 0" false false)
      (else
        (Transformation|SetRelativeRotation (Variables|Default|GetSprite) "0.000000,180.000000,0.000000" false false))))
  (:Completed
    (if (not (Variables|Default|GetIsJumping?))
      (Sprite|SetFlipbook (Variables|Default|GetSprite) "/Game/Art/Character/FB_Idle.FB_Idle"))))

(event Input|EnhancedActionEvents|EnhancedInputActionIA_Jump
  (params (ActionValue :type Boolean) (ElapsedSeconds :type Float%20%28double-precision%29) (TriggeredSeconds :type Float%20%28double-precision%29) (InputAction :type Input%20Action%20Object%20Reference :default "/Game/Inputs/InputActions/IA_Jump.IA_Jump"))
  (:Started
    (Variables|Default|SetIsJumping? true)
    (Character|Jump)
    (Sprite|SetFlipbook (Variables|Default|GetSprite) "/Game/Art/Character/FB_Jump.FB_Jump"))
  (:Completed
    (Character|StopJumping)))

(event EventBeginPlay)

(event Collision|EventActorBeginOverlap
  (params (OtherActor :type Actor%20Object%20Reference)))

(event EventTick
  (params (DeltaSeconds :type Float%20%28single-precision%29)))

(event EventOnLanded
  (params (Hit :type Hit%20Result%20Structure%20%28by%20ref%29))
  (Sprite|SetFlipbook (Variables|Default|GetSprite) "/Game/Art/Character/FB_Idle.FB_Idle")
  (Variables|Default|SetIsJumping? false))

(event Input|KeyboardEvents|E
  (params (Key :type Key%20Structure :default "None"))
  (:Pressed
    (for _array_element (Collision|GetOverlappingActors (Variables|Default|GetSphere) "/Game/Blueprints/Interactables/BP_Interactable.BP_Interactable_C" :!class /Script/Engine.PrimitiveComponent)
      (bind _asbp_interactable (Utilities|Casting|CastToBP_Interactable _array_element))
      (Default|Interact _asbp_interactable))))

(fn ConstructionScript)