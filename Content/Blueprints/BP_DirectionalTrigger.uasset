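; Directional trigger box that messages linked actors according to which side the third-person character enters or leaves from.
; On begin and end overlap, it compares the character's distance to red and green arrow markers to pick that side's actor map.
; It then calls TriggerMessage on each mapped actor, passing the inverse of its stored boolean on entry and the stored value on exit.
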(event OnComponentBeginOverlap(Box)
  (params (OverlappedComponent :type Primitive%20Component%20Object%20Reference) (OtherActor :type Actor%20Object%20Reference) (OtherComp :type Primitive%20Component%20Object%20Reference) (OtherBodyIndex :type Integer) (bFromSweep :type Boolean) (SweepResult :type Hit%20Result%20Structure%20%28by%20ref%29))
  (bind _asbp_third_person_character (Utilities|Casting|CastToBP_ThirdPersonCharacter OtherActor))
  (if (< (Math|Vector|Distance(Vector) (Transformation|GetActorLocation _asbp_third_person_character) (Transformation|GetWorldLocation (Variables|Default|GetRedArrow))) (Math|Vector|Distance(Vector) (Transformation|GetActorLocation _asbp_third_person_character) (Transformation|GetWorldLocation (Variables|Default|GetGreenArrow))))
    (bind (_keypin _valuepin) (Utilities|Map|ForEachLoop(Map) (Variables|Default|GetRedActorsToActivate))
      (:then
        (Class|BPITrigger|Trigger(Message) _keypin (not _valuepin))))
    (else
      (bind (_keypin_2 _valuepin_2) (Utilities|Map|ForEachLoop(Map) (Variables|Default|GetGreenActorsToActivate))
        (:then
          (Class|BPITrigger|Trigger(Message) _keypin_2 (not _valuepin_2)))))))

(event OnComponentEndOverlap(Box)
  (params (OverlappedComponent :type Primitive%20Component%20Object%20Reference) (OtherActor :type Actor%20Object%20Reference) (OtherComp :type Primitive%20Component%20Object%20Reference) (OtherBodyIndex :type Integer))
  (bind _asbp_third_person_character (Utilities|Casting|CastToBP_ThirdPersonCharacter OtherActor))
  (if (< (Math|Vector|Distance(Vector) (Transformation|GetActorLocation _asbp_third_person_character) (Transformation|GetWorldLocation (Variables|Default|GetRedArrow))) (Math|Vector|Distance(Vector) (Transformation|GetActorLocation _asbp_third_person_character) (Transformation|GetWorldLocation (Variables|Default|GetGreenArrow))))
    (bind (_keypin _valuepin) (Utilities|Map|ForEachLoop(Map) (Variables|Default|GetRedActorsToActivate))
      (:then
        (Class|BPITrigger|Trigger(Message) _keypin _valuepin)))
    (else
      (bind (_keypin_2 _valuepin_2) (Utilities|Map|ForEachLoop(Map) (Variables|Default|GetGreenActorsToActivate))
        (:then
          (Class|BPITrigger|Trigger(Message) _keypin_2 _valuepin_2))))))

(fn ConstructionScript)