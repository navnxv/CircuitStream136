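; BP_NPC is a Paper2D flipbook character that walks back and forth on its own and dies when the player overlaps its death box.
; Tick constantly applies forward movement input, and the actor rotates 180 degrees when its wall box begins an overlap or its surface box ends one.
; On death it disables collision and tick, plays a death flipbook, then switches to a looping dead flipbook after a short delay.
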(event OnComponentBeginOverlap(WallDetectionBox)
  (params (OverlappedComponent :type Primitive%20Component%20Object%20Reference) (OtherActor :type Actor%20Object%20Reference) (OtherComp :type Primitive%20Component%20Object%20Reference) (OtherBodyIndex :type Integer) (bFromSweep :type Boolean) (SweepResult :type Hit%20Result%20Structure%20%28by%20ref%29))
  (Class|Actor|AddActorWorldRotation "0.000000,180.000000,0.000000"))

(event OnComponentEndOverlap(SurfaceDetectionBox)
  (params (OverlappedComponent :type Primitive%20Component%20Object%20Reference) (OtherActor :type Actor%20Object%20Reference) (OtherComp :type Primitive%20Component%20Object%20Reference) (OtherBodyIndex :type Integer))
  (Class|Actor|AddActorWorldRotation "0.000000,180.000000,0.000000"))

(event OnComponentBeginOverlap(DeathBox)
  (params (OverlappedComponent :type Primitive%20Component%20Object%20Reference) (OtherActor :type Actor%20Object%20Reference) (OtherComp :type Primitive%20Component%20Object%20Reference) (OtherBodyIndex :type Integer) (bFromSweep :type Boolean) (SweepResult :type Hit%20Result%20Structure%20%28by%20ref%29))
  (Utilities|Casting|CastToBP_PlayerCharacter OtherActor)
  (Sprite|SetFlipbook (Variables|Default|GetSprite) "/Game/Art/GenericCharacters/red/FB_Dead.FB_Dead")
  (Collision|SetCollisionEnabled (Variables|Collision|GetCapsuleComponent) "NoCollision")
  (Actor|Tick|SetActorTickEnabled false)
  (Utilities|FlowControl|Delay 1.2)
  (Sprite|SetFlipbook (Variables|Default|GetSprite) "/Game/Art/GenericCharacters/red/FB_DeadLoop.FB_DeadLoop"))

(event EventTick
  (params (DeltaSeconds :type Float%20%28single-precision%29))
  (Pawn|Input|AddMovementInput (Transformation|GetActorForwardVector) 1.0 false))

(fn ConstructionScript)